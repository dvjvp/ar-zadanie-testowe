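; Rifle fire ability that shoots repeated series of shots while the hold-fire input is active, gated by an active flag.
; Activation starts an initial-delay timer, and the Shot event schedules further timers with separate delays within and between series.
; Each shot fires from the muzzle along control rotation and uses one ammo; empty ammo skips firing without blocking activation.
; Cancelling clears the active flag and the stored shot timer.
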(event Custom|Shot
  (Utilities|FlowControl|Sequence
    (:then_0
      (if (> (Class|ShootingAbility|GetAmmoCount) 0)
        (bind _aspawn (Utilities|Casting|CastToPawn (Components|GetOwner)))
        (Class|ShootingAbility|FireWeapon (Class|ShootingAbility|GetMuzzleLocation) (Math|Vector|GetForwardVector (Pawn|GetControlRotation _aspawn :!class /Script/Engine.Pawn)))
        (Class|ShootingAbility|UseAmmo 1)))
    (:then_1
      (bind _result (Math|Integer|IncrementInt (Variables|Default|GetLastShotIdx))
        (:%20%20
          (if (>= _result (Variables|Default|GetNumShotsInSeries))
            (Variables|Default|SetLastShotIdx 0)
            (Utilities|Time|SetTimerbyEvent (EventDispatchers|CreateEvent :!event Custom|Shot) (Variables|Default|GetDelayAfterEachSeries))
            (else
              (Utilities|Time|SetTimerbyEvent (EventDispatchers|CreateEvent :!event Custom|Shot) (Variables|Default|GetDelayBetweenShotsInSeries)))))))))

(event Input|EnhancedActionEvents|EnhancedInputActionIA_Fire_Hold
  (params (ActionValue :type Boolean) (ElapsedSeconds :type Float%20%28double-precision%29) (TriggeredSeconds :type Float%20%28double-precision%29) (InputAction :type Input%20Action%20Object%20Reference :default "/Game/Input/Actions/IA_Fire_Hold.IA_Fire_Hold"))
  (:Started
    (if (CallFunction|CanbeActivated)
      (Class|PlayerAbility|TrytoActivate) ; Allow to activate even at 0 ammo. There won't be any shots tho\n(would use a different animation or sth to show it)
      (Development|PrintString "IA_FIRE: START")))
  (:Completed
    (if (CallFunction|CanbeCanceled)
      (Class|PlayerAbility|TrytoCancel)
      (Development|PrintString "IA_FIRE: STOP"))))

(event EventOnActivated
  (Variables|Default|SetAbilityIsActive true)
  (Variables|Default|SetLastShotIdx -1)
  (bind _returnvalue (Utilities|Time|SetTimerbyEvent (EventDispatchers|CreateEvent :!event Custom|Shot) (Variables|Default|GetInitialDelay)))
  (Variables|Default|SetShot%20Timer _returnvalue))

(event EventOnCanceled
  (params (Reason :type EAbilityCancelReason%20Enum :default "CanceledByGameCode"))
  (bind _shot_timer (Variables|Default|GetShot%20Timer))
  (Variables|Default|SetAbilityIsActive false)
  (Utilities|Time|PauseTimerbyHandle _shot_timer)
  (Utilities|Time|ClearandInvalidateTimerbyHandle _shot_timer))

(fn CanbeCanceled
  (return (and (|CallParentFunction) (Variables|Default|GetAbilityIsActive))))

(fn CanbeActivated
  (return (and (|CallParentFunction) (not (Variables|Default|GetAbilityIsActive)))))