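; Base Blueprint for a pickup spawner that displays its cooldown progress on a plane component.
; On BeginPlay it creates a dynamic material instance from CooldownPlane's material and assigns it back to the plane.
; Each tick it shows the plane only during cooldown, feeding GetCooldownProgress into the material's PercentFilled parameter.
; Cooldown state comes from functions defined outside these graphs, which contain no spawning logic.
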(event EventBeginPlay
  (bind _returnvalue (Rendering|Material|CreateDynamicMaterialInstance (Rendering|Material|GetMaterial (Variables|Default|GetCooldownPlane) 0) "None" "None" :!class /Script/Engine.KismetMaterialLibrary))
  (bind _output_get (Variables|Default|SetCooldownDynamicMaterial _returnvalue))
  (Rendering|Material|SetMaterial (Variables|Default|GetCooldownPlane) 0 _output_get))

(event EventTick
  (params (DeltaSeconds :type Float%20%28single-precision%29))
  (bind _returnvalue (Class|PickupSpawnerBase|IsonCooldown))
  (Development|SetHiddeninGame (Variables|Default|GetCooldownPlane) (not _returnvalue) false)
  (if _returnvalue
    (Rendering|Material|SetScalarParameterValue (Variables|Default|GetCooldownDynamicMaterial) "PercentFilled" (Class|PickupSpawnerBase|GetCooldownProgress) :!class /Script/Engine.MaterialInstanceDynamic)))

(fn ConstructionScript)