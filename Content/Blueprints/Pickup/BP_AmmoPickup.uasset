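; Ammo pickup that gives whatever ammo type the collecting pawn's current weapon uses, in that weapon's pickup amount.
; It finds the weapon class through the pawn's EquipmentComponent and reads ammo type and amount from its class defaults.
; On pickup it writes both into InventoryItem and NumToAdd, then runs the parent effect.
; Pickup is allowed only when that ammo type is valid and the pawn's InventoryComponent can add it.
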(event EventApplyPickupEffect
  (params (ToActor :type Actor%20Object%20Reference))
  ;[0.15 0.15 0.15 0.5] Automatically change the ammo type and amount to match the current weapon
  (bind (_ammo_type _num_ammo_given_on_pickup) (CallFunction|GetCurrentAmmoType ToActor))
  (Variables|Default|SetInventoryItem _ammo_type)
  (Variables|Default|SetNumToAdd _num_ammo_given_on_pickup)
  (|CallParentFunction ToActor))

(fn ConstructionScript
  (|CallParentFunction))

(fn CanbePickedUp
  (params (ByActor :type Actor%20Object%20Reference))
  (bind _returnvalue (Actor|GetComponentbyClass ByActor "/Script/Survival.InventoryComponent"))
  (bind _ammo_type (CallFunction|GetCurrentAmmoType ByActor))
  (if (Utilities|IsValidClass _ammo_type)
    (Utilities|Casting|CastToPawn ByActor
      (:then
        (Utilities|IsValid _returnvalue
          (:Is%20Valid
            (return (Class|InventoryComponent|CanAddItems _returnvalue _ammo_type)))
          (:Is%20Not%20Valid
            _)))
      (:CastFailed
        _)))
  (return false))

(fn GetCurrentWeapon
  (params (FromActor :type Actor%20Object%20Reference))
  (bind _aspawn (Utilities|Casting|CastToPawn FromActor)
    (:then
      (Utilities|IsValid (Actor|GetComponentbyClass _aspawn "/Script/Survival.EquipmentComponent")
        (:Is%20Valid
          (return (Class|EquipmentComponent|GetCurrentWeapon (Actor|GetComponentbyClass _aspawn "/Script/Survival.EquipmentComponent"))))
        (:Is%20Not%20Valid
          _)))
    (:CastFailed
      _))
  (return 0))

(fn GetCurrentAmmoType
  (params (FromActor :type Actor%20Object%20Reference))
  (bind _returnvalue (CallFunction|GetCurrentWeapon FromActor))
  (if (Utilities|IsValidClass _returnvalue)
    (return (.AmmoType (Utilities|GetClassDefaults _returnvalue)) (.AmmoGivenOnPickup (Utilities|GetClassDefaults _returnvalue)))
    (else
      (return 0 0))))